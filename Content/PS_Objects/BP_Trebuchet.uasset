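; BP_Trebuchet is an interactable trebuchet that launches a physically roped projectile.
; Each Interact alternates between slowly winding the pull arm back to arm it and quickly swinging it forward to fire.
; While firing, Tick watches the projectile's position in actor space and, once it crosses local Y zero, breaks the rope constraint, frees the cable end and detaches the projectile.
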(event `/Game/BPI_Interact.Interact`
  (bind _bp_trebuchet_pullarm (`self.BP_Trebuchet_PullArm`))
  (bind _bp_trebuchet_pullarm_2 (`self.BP_Trebuchet_PullArm`))
  (if (`self.bArmed?`)
    (set `self.bFire?` true)
    (`KismetSystemLibrary.MoveComponentTo` _bp_trebuchet_pullarm (`SceneComponent.RelativeLocation` _bp_trebuchet_pullarm) (struct) false false 0.5)
    (set `self.bArmed?` false)
    (else
      (set `self.bFire?` false)
      (`KismetSystemLibrary.MoveComponentTo` _bp_trebuchet_pullarm_2 (`SceneComponent.RelativeLocation` _bp_trebuchet_pullarm_2) (struct :`Roll` -110.0) false false 2.0)
      (set `self.bArmed?` true))))

(event `self.ReceiveTick`
  (params (DeltaSeconds :type "Float (single-precision)"))
  (if (`self.bFire?`)
    (if (>= (.y (`KismetMathLibrary.InverseTransformLocation` (`self.GetTransform`) (`SceneComponent.K2_GetComponentLocation` (`self.Projectile`)))) 0.0)
      (`/Engine/EditorBlueprintResources/StandardMacros.DoOnce` false :!label _label
        (:`Completed`
          (`PhysicsConstraintComponent.BreakConstraint` (`self.ProjectileRope`))
          (set `CableComponent.bAttachEnd` false (`self.Cable`))
          (`SceneComponent.K2_DetachFromComponent` (`self.Projectile`) "KeepWorld" "KeepWorld" "KeepWorld" true)
          (set `CableComponent.bEnableCollision` true (`self.Cable`))))
      (else
        (goto _label :!via `Reset`)))))

(fn `UserConstructionScript`)