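; BP_Crankhaft is a physics-driven crankshaft whose Wheel can be motorized through the WheelAxis constraint.
; When Rotate is set, the construction script enables a swing velocity drive on WheelAxis, using MotorStrenght as strength and AngularVelocity as the Y-axis target.
; On BeginPlay, it offsets the Wheel's center of mass by the negated local center of mass, shifting it toward the component's pivot.
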(event `self.ReceiveBeginPlay`
  (bind _wheel (`self.Wheel`))
  (`PrimitiveComponent.SetCenterOfMass` (`self.Wheel`) (`KismetMathLibrary.NegateVector` (`KismetMathLibrary.InverseTransformLocation` (`SceneComponent.K2_GetComponentToWorld` _wheel) (`PrimitiveComponent.GetCenterOfMass` _wheel "None"))) "None"))

(fn `UserConstructionScript`
  (bind _wheelaxis (`self.WheelAxis`))
  (if (`self.bRotate?`)
    (`PhysicsConstraintComponent.SetAngularDriveParams` _wheelaxis 0.0 (`self.Motor Strenght`) 0.0)
    (`PhysicsConstraintComponent.SetAngularVelocityDriveTwistAndSwing` _wheelaxis false true)
    (`PhysicsConstraintComponent.SetAngularVelocityTarget` _wheelaxis (`KismetMathLibrary.MakeVector` 0.0 (`self.Angular Velocity`)))))