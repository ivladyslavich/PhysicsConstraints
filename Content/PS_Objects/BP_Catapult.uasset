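; BP_Catapult is a physics-driven catapult that toggles its arm on each Interact event.
; A FlipFlop alternates the Spring constraint's angular drive between a very stiff swing to one pitch target and a far softer return to the opposite one.
; Each toggle wakes the Arm's rigid body so the physics simulation responds to the new drive.
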(event `self.ReceiveBeginPlay`)

(event `/Game/BPI_Interact.Interact`
  (bind _spring (`self.Spring`))
  (`/Engine/EditorBlueprintResources/StandardMacros.FlipFlop`
    (:`A`
      (`PhysicsConstraintComponent.SetAngularOrientationTarget` (`self.Spring`) (`KismetMathLibrary.MakeRotator` 0.0 45.0))
      (`PhysicsConstraintComponent.SetAngularDriveParams` _spring 2500.0 1.0 0.0))
    (:`B`
      (`PhysicsConstraintComponent.SetAngularOrientationTarget` (`self.Spring`) (`KismetMathLibrary.MakeRotator` 0.0 -45.0))
      (`PhysicsConstraintComponent.SetAngularDriveParams` _spring 25.0 1.0 0.0)
      (`PhysicsConstraintComponent.SetAngularDriveParams` (`self.Spring`) 25.0 1.0 0.0)))
  (`PrimitiveComponent.WakeRigidBody` (`self.Arm`) "None"))

(fn `UserConstructionScript`)