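; BP_RopeBridge is a procedural physics rope bridge whose planks run from the Step component toward EndPoint.
; The Construction Script aims Step at EndPoint, then chains NumbOfElemen static mesh planks at even intervals along that line.
; Each plank is joined to the previous one by left and right physics constraints offset along its right vector.
; The final plank has physics simulation turned off, and the event graph holds no logic.
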(fn `CreatePC`
  (params (InTransform :type "Transform Structure (by ref)") (Component1 :type "PrimitiveComponent Object Reference") (Component2 :type "PrimitiveComponent Object Reference") (LeftPC :type Boolean))
  (bind _returnvalue (`KismetMathLibrary.GetRightVector` InTransform_Rotation))
  (bind _returnvalue_2 (`AddComponent|NODE_AddPhysicsConstraintComponent-0` :`RelativeTransform` (`KismetMathLibrary.MakeTransform` (+ (* (select `bool` LeftPC :`false` (* _returnvalue -1.0) :`true` _returnvalue) 70.0) InTransform_Location) InTransform_Rotation)))
  (`PhysicsConstraintComponent.SetConstrainedComponents` _returnvalue_2 Component1 "None" Component2 "None"))

(fn `CreateStaticMesh`
  (params (InTransform :type "Transform Structure (by ref)"))
  (returns (val :type "StaticMeshComponent Object Reference"))
  (bind _returnvalue (`AddComponent|NODE_AddStaticMeshComponent-0` :`RelativeTransform` (`KismetMathLibrary.MakeTransform` (+ InTransform_Location (* (`KismetMathLibrary.GetDirectionUnitVector` (0.0 0.0 0.0) (`self.EndPoint`)) (/ (`KismetMathLibrary.VSize` (`self.EndPoint`)) (`KismetMathLibrary.Conv_IntToDouble` (`self.NumbOfElemen`))))) InTransform_Rotation InTransform_Scale)))
  (return _returnvalue))

(fn `UserConstructionScript`
  (bind _lastplank (`self.LastPlank`))
  (bind _returnvalue (`SceneComponent.GetRelativeTransform` _lastplank))
  (`SceneComponent.K2_SetRelativeRotation` (`self.Step`) (`KismetMathLibrary.FindLookAtRotation` (0.0 0.0 0.0) (`self.EndPoint`)) false true)
  (set `self.LastPlank` (`self.Step`))
  (for _ (range 1 (+ (`self.NumbOfElemen`) 1))
    (bind _val (`self.CreateStaticMesh` _returnvalue))
    (`self.CreatePC` _returnvalue _val _lastplank true)
    (`self.CreatePC` _returnvalue _val _lastplank)
    (set `self.LastPlank` _val))
  (`PrimitiveComponent.SetSimulatePhysics` (`self.LastPlank`) false))